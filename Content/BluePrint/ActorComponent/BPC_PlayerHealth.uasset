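; Actor component that tracks a player's health and notifies listeners when it changes or runs out.
; IncreaseHealth adds an amount clamped between zero and a fixed maximum, then fires the UpdatedHealth dispatcher.
; DecreaseHealth subtracts damage without clamping, fires UpdatedHealth, then fires the Dead dispatcher whenever health is at or below zero.
; The event graph is empty.
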(fn `DecreaseHealth`
  (params (Damage :type "Float (double-precision)"))
  (set `self.Health` (- (`self.Health`) Damage))
  (`self.UpdatedHealth`)
  (if (<= (`self.Health`) 0.0)
    (`self.Dead`)))

(fn `IncreaseHealth`
  (params (Amount :type "Float (double-precision)"))
  (set `self.Health` (`KismetMathLibrary.FClamp` (+ (`self.Health`) Amount) 0.0 100.0))
  (`self.UpdatedHealth`))