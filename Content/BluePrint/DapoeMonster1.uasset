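; DapoeMonster1 is a monster actor with an intro rotation and a health bar widget.
; On BeginPlay it spawns a MoveCircle at one of its transforms, then after a short delay plays a timeline that lerps its rotation from zero to a fixed 45-degree angle.
; Tick casts the widget to WBP_HealthBar and sets its percent from Health on a 100-point scale.
; No damage or overlap logic runs here.
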(event `self.ReceiveBeginPlay`
  (`|SpawnActorFromClass` "/Game/BluePrint/MoveCircle.MoveCircle_C" (`SceneComponent.K2_GetComponentToWorld` (`self.1`)) "AlwaysSpawn" "MultiplyWithRoot" null null)
  (`KismetSystemLibrary.Delay` 3.5)
  (bind (_direction _newtrack_0) (`Timeline|Timeline` :`NewTime` 0.0)
    (:`Update`
      (`self.K2_SetActorRotation` (`KismetMathLibrary.RLerp` (struct) (struct :`Yaw` -45.0) _newtrack_0)))))

(event `self.ReceiveTick`
  (params (DeltaSeconds :type "Float (single-precision)"))
  (bind _aswbp_health_bar (cast `/Game/BluePrint/WB_Bp/WBP_HealthBar` (`WidgetComponent.GetWidget` (`self.HealthBarWidget`))))
  (`ProgressBar.SetPercent` (`/Game/BluePrint/WB_Bp/WBP_HealthBar.Health_Bar` _aswbp_health_bar) (/ (`self.health`) 100.0)))

(fn `UserConstructionScript`)