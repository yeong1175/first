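; Phase 1 enemy monster that runs a timed charge-and-spawn opening, then chases the player.
; BeginPlay chains delays, the charge montage and two rotation timelines to spawn MoveCircle1 and MoveCircle2.
; Tick turns it toward the player each frame and, after a set elapsed time, plays Dora and starts AIMoveTo when the player is distant, re-arming on success.
; Click and deselect events toggle an outline overlay material.
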(event `self.ReceiveBeginPlay`
  (bind _returnvalue_location (`KismetMathLibrary.BreakTransform` (`SceneComponent.K2_GetComponentToWorld` (`self.Body`))))
  (`self.PlayAnimMontage` "/Game/MakeAnimSequence/Charge1Montague.Charge1Montague")
  (`KismetSystemLibrary.Delay` 4.39)
  (`|SpawnActorFromClass` "/Game/BluePrint/Phase1Enemy/MoveCircle1.MoveCircle1_C" (`KismetMathLibrary.MakeTransform` (+ _returnvalue_location (100.0 0.0 0.0))) "AlwaysSpawn" "MultiplyWithRoot" null null)
  (`KismetSystemLibrary.Delay` 3.5)
  (bind (_direction _newtrack_0) (`Timeline|Timeline`)
    (:`Update`
      (`self.K2_SetActorRotation` (`KismetMathLibrary.RLerp` (struct) (struct :`Yaw` -45.0) _newtrack_0))
      (`KismetSystemLibrary.Delay` 6.0)
      (bind (_direction_2 _newtrack_0_2) (`Timeline|Timeline_0`)
        (:`Update`
          (`self.K2_SetActorRotation` (`KismetMathLibrary.RLerp` (struct :`Yaw` -45.0) (struct :`Pitch` 30.0 :`Yaw` -45.0) _newtrack_0_2))
          (`KismetSystemLibrary.Delay` 1.0)
          (`self.PlayAnimMontage` "/Game/MakeAnimSequence/Charge1Montague.Charge1Montague")
          (`KismetSystemLibrary.Delay` 8.0)
          (`self.StopAnimMontage` "/Game/MakeAnimSequence/Charge1Montague.Charge1Montague")
          (`|SpawnActorFromClass` "/Game/BluePrint/Phase1Enemy/MoveCircle2.MoveCircle2_C" (`SceneComponent.K2_GetComponentToWorld` (`self.Body`)) "AlwaysSpawn" "MultiplyWithRoot" null null))))))

(event `self.ReceiveTick`
  (params (DeltaSeconds :type "Float (single-precision)"))
  (`|ExecutionSequence`
    (:`then_1`
      (`self.K2_SetActorRotation` (`KismetMathLibrary.FindLookAtRotation` (`self.K2_GetActorLocation`) (`self.K2_GetActorLocation` (`GameplayStatics.GetPlayerPawn` 0)))))
    (:`then_2`
      (bind _output_get (set `self.elpasedtime` (+ (`self.elpasedtime`) DeltaSeconds)))
      (`|ExecutionSequence`
        (:`then_0`
          (if (and (> _output_get 42.0) (> (`KismetMathLibrary.VSize` (- (`self.K2_GetActorLocation` (`GameplayStatics.GetPlayerPawn` 0)) (`self.K2_GetActorLocation`))) 600.0))
            (`/Engine/EditorBlueprintResources/StandardMacros.DoOnce` false :!label _label
              (:`Completed`
                (`self.PlayAnimMontage` "/Game/MakeAnimSequence/dora.dora")
                (`|AIMoveTo` self (0.0 0.0 0.0) (`GameplayStatics.GetPlayerCharacter` 0) 50.0 true
                  (:`OnSuccess`
                    (goto _label :!via `Reset`)))))))))))

(event `/Game/BPI_Test/Clicked.OnClickEvent`
  (bind _mesh (`self.Mesh`))
  (`MeshComponent.SetOverlayMaterial` _mesh "/Game/material/Outline/ClickOutline.ClickOutline")
  (`SceneComponent.SetVisibility` _mesh true false))

(event `/Game/BPI_Test/Clicked.OnDeselecEvent`
  (bind _mesh (`self.Mesh`))
  (`MeshComponent.SetOverlayMaterial` _mesh null)
  (`SceneComponent.SetVisibility` _mesh true false))

(fn `UserConstructionScript`)