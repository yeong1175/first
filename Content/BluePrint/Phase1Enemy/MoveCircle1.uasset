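; Phase 1 enemy movement actor that loops around a small square path for about 39 seconds, then destroys itself.
; Tick passes through a gate into Phase1, which applies a local offset scaled by BojungSpeed and delta time, cycling through four perpendicular directions every half second.
; A total elapsed counter sets a flag named "10", closes the gate and destroys the actor.
; The looping BeginPlay timer calls an empty Domove event.
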(event `self.ReceiveTick`
  (params (DeltaSeconds :type "Float (single-precision)"))
  (`|ExecutionSequence`
    (:`then_0`
      (`/Engine/EditorBlueprintResources/StandardMacros.Gate` false :!label _label
        (:`Exit`
          (`self.Phase1` DeltaSeconds DeltaSeconds))))
    (:`then_1`
      (bind _output_get (set `self.WholeElapsed` (+ DeltaSeconds (`self.WholeElapsed`))))
      (if (> _output_get 39.0)
        (set `self.1_0` true)
        (`|ExecutionSequence`
          (:`then_0`
            (goto _label :!via `Close`))
          (:`then_1`
            (`self.K2_DestroyActor`)))))))

(event `self.ReceiveBeginPlay`
  (`KismetSystemLibrary.K2_SetTimerDelegate` (delegate `Domove`) 0.01 true))

(event `Domove`)

(fn `Phase1`
  (params (C :type "Float (single-precision)") (B :type "Float (double-precision)"))
  (`self.K2_AddActorLocalOffset` self (* (select `int` (`self.StepCount`) :`0` (0.0 -21.0 0.0) :`1` (21.0 0.0 0.0) :`2` (0.0 21.0 0.0) :`3` (-21.0 0.0 0.0) :!type "Vector Structure") (`self.BojungSpeed`) C) false false)
  (bind _output_get (set `self.ElapsedTime` (+ (`self.ElapsedTime`) B)))
  (if (> _output_get 0.5)
    (set `self.StepCount` (mod (+ (`self.StepCount`) 1) 4))
    (set `self.ElapsedTime` 0.0)))

(fn `UserConstructionScript`)