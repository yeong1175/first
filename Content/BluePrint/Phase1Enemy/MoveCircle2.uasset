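; Phase 1 enemy actor that moves to a fixed high point, swells, descends and explodes.
; BeginPlay chains three timelines with delays: lerp movement while spawning effects every update, scale up from zero, then drop to a lower point.
; A delayed explosion matching the actor's scale precedes its destruction.
; A separate Phase1 function, uncalled here, steps local offsets through four directions on a half-second timer, tracing a square.
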(event `self.ReceiveBeginPlay`
  (bind (_direction _newtrack_0) (`Timeline|Timeline`)
    (:`Update`
      (`self.K2_SetActorLocation` (`KismetMathLibrary.VLerp` (`self.K2_GetActorLocation`) (50.0 -50.0 900.0) _newtrack_0))
      (`self.SetActorScale3D` (1.0 1.0 1.0))
      (`NiagaraFunctionLibrary.SpawnSystemAtLocation` "/Game/material/AttackEffect/Fx.Fx" (`self.K2_GetActorLocation`))
      (`KismetSystemLibrary.Delay` 7.0)
      (bind (_direction_2 _newtrack_0_2) (`Timeline|Timeline_1`)
        (:`Update`
          (`self.SetActorScale3D` (`KismetMathLibrary.VLerp` (0.0 0.0 0.0) (8.5 8.5 8.5) _newtrack_0_2)))
        (:`Finished`
          (`KismetSystemLibrary.Delay` 3.0)
          (bind (_direction_3 _newtrack_0_3) (`Timeline|Timeline_0`)
            (:`Update`
              (`self.K2_SetActorLocation` (`KismetMathLibrary.VLerp` (`self.K2_GetActorLocation`) (50.0 -50.0 300.0) _newtrack_0_3))
              (`KismetSystemLibrary.Delay` 3.0)
              (`GameplayStatics.SpawnEmitterAtLocation` "/Game/StarterContent/Particles/P_Explosion.P_Explosion" (`self.K2_GetActorLocation`) (struct) (`self.GetActorScale3D`))
              (`self.K2_DestroyActor`))))))))

(fn `Phase1`
  (params (C :type "Float (single-precision)") (B :type "Float (double-precision)"))
  (`self.K2_AddActorLocalOffset` self (* (select `int` (`self.StepCount`) :`0` (21.0 0.0 0.0) :`1` (0.0 -21.0 0.0) :`2` (-21.0 0.0 0.0) :`3` (0.0 21.0 0.0) :!type "Vector Structure") (`self.BojungSpeed`) C) false false)
  (bind _output_get (set `self.ElapsedTime` (+ (`self.ElapsedTime`) B)))
  (if (> _output_get 0.5)
    (set `self.StepCount` (mod (+ (`self.StepCount`) 1) 4))
    (set `self.ElapsedTime` 0.0)))

(fn `UserConstructionScript`)