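; Parent enemy for the Phase 1 circle enemies that wanders at random and can be visually highlighted when clicked.
; From BeginPlay it loops AI MoveTo toward random reachable points around its current location, pausing briefly after each success or failure.
; Click and deselect events apply and clear an outline overlay material on the mesh.
; The box overlap only casts to the third-person character, with no further action.
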(event `self.ReceiveBeginPlay`
  (`|AIMoveTo` self (`NavigationSystemV1.K2_GetRandomReachablePointInRadius` (`self.K2_GetActorLocation`) 500.0 null null) null 50.0 :!label _label
    (:`OnSuccess`
      _)
    (:`OnFail`
      _))
  (`KismetSystemLibrary.Delay` 1.0)
  (goto _label))

(event `self.Box.OnComponentBeginOverlap`
  (params (OverlappedComponent :type "PrimitiveComponent Object Reference") (OtherActor :type "Actor Object Reference") (OtherComp :type "PrimitiveComponent Object Reference") (OtherBodyIndex :type Integer) (bFromSweep :type Boolean) (SweepResult :type "HitResult Structure (by ref)"))
  (cast `/Game/ThirdPerson/Blueprints/BP_ThirdPersonCharacter` OtherActor))

(event `self.ReceiveTick`
  (params (DeltaSeconds :type "Float (single-precision)")))

(event `self.OnClickEvent`
  (bind _mesh (`self.Mesh`))
  (`MeshComponent.SetOverlayMaterial` _mesh "/Game/material/Outline/ClickOutline.ClickOutline")
  (`SceneComponent.SetVisibility` _mesh true false))

(event `self.OnDeselecEvent`
  (`MeshComponent.SetOverlayMaterial` (`self.Mesh`) null)
  (`SceneComponent.SetVisibility` (`self.Mesh`) true false))

(fn `UserConstructionScript`)