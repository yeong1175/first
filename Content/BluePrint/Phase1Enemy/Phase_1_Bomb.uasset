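; Phase 1 enemy bomb actor that explodes on a timer after spawning and damages nearby pawns.
; BeginPlay waits, spawns a scaled explosion emitter, then passes a DoOnce into a second delay and a second explosion.
; Only the second blast runs a sphere overlap for pawns and applies damage to each, resetting the DoOnce inside the loop.
; Nothing loops back to repeat the sequence or destroys the actor.
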(event `self.ReceiveBeginPlay`
  (`|ExecutionSequence`
    (:`then_0`
      (`KismetSystemLibrary.Delay` 3.0)
      (`GameplayStatics.SpawnEmitterAtLocation` "/Game/StarterContent/Particles/P_Explosion.P_Explosion" (`self.K2_GetActorLocation`) (struct) (3.0 3.0 3.0))
      (`/Engine/EditorBlueprintResources/StandardMacros.DoOnce` false :!label _label
        (:`Completed`
          (`KismetSystemLibrary.Delay` 3.0)
          (`GameplayStatics.SpawnEmitterAtLocation` "/Game/StarterContent/Particles/P_Explosion.P_Explosion" (`self.K2_GetActorLocation`) (struct) (3.0 3.0 3.0))
          (bind _outactors (`KismetSystemLibrary.SphereOverlapActors` (`self.K2_GetActorLocation`) 500.0 (`|MakeArray` "ObjectTypeQuery3" :!type "EObjectTypeQuery Enum")))
          (for _array_element _outactors
            (`GameplayStatics.ApplyDamage` _array_element 50.0)
            (goto _label :!via `Reset`)))))))

(fn `UserConstructionScript`)