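; Actor in the Phase 1 enemy folder whose static mesh is configured by an enum-keyed data map; its gameplay role is not shown.
; The construction script looks up TestEnum in TestEnum2 to set the mesh, a dynamic material and uniform world scale.
; It also passes the entry's color to a vector parameter named None.
; The event graph does nothing at runtime, holding only empty events and disconnected material and scale nodes.
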(event `self.ReceiveBeginPlay`)

(fn `UserConstructionScript`
  (bind _value (`BlueprintMapLibrary.Map_Find` (`self.TestEnum2`) (`self.TestEnum`)))
  (`StaticMeshComponent.SetStaticMesh` (`self.StaticMesh`) (`.MemberVar_7_11_23428878443B5F258ED8D693C28AB5C1` (break `/Game/Structure/AttackDamage` _value)))
  (bind _returnvalue (`PrimitiveComponent.CreateDynamicMaterialInstance` (`self.StaticMesh`) 0 "/Game/material/TesThoric/4_Mat.4_Mat" "None"))
  (`PrimitiveComponent.SetMaterial` (`self.StaticMesh`) 0 _returnvalue)
  (`KismetMaterialLibrary.SetVectorParameterValue` null "None" (break `/Game/Structure/AttackDamage` _value))
  (`SceneComponent.SetWorldScale3D` (`self.StaticMesh`) (`KismetMathLibrary.MakeVector` (`.MemberVar_8_12_DE86A3F04904003FCD2F7493C30CC360` (break `/Game/Structure/AttackDamage` _value)) (`.MemberVar_8_12_DE86A3F04904003FCD2F7493C30CC360` (break `/Game/Structure/AttackDamage` _value)) (`.MemberVar_8_12_DE86A3F04904003FCD2F7493C30CC360` (break `/Game/Structure/AttackDamage` _value)))))