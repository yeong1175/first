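; Inventory component Blueprint that stores picked-up item data for its owning actor.
; AddItem looks up the given ID in the pickup data table and, when found, appends the row to the DatatableItems array and prints its ChestID.
; ShowInventorylist loops over the stored rows and prints each ChestID as debug output.
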(event `AddItem`
  (params (In_ItemID :type Name))
  (bind _returnvalue (`|GetDataTableRow` "/Game/Structure/DataTable/PickupDataTabel.PickupDataTabel" In_ItemID)
    (:`then`
      (`KismetArrayLibrary.Array_Add` (`self.DatatableItems`) _returnvalue)
      (`KismetSystemLibrary.PrintString` (`KismetStringLibrary.Conv_NameToString` (`.ChestID_8_BFBAAD3F4112D46E9C599BBFA1B441CD` (break `/Game/Structure/S_ChestData` _returnvalue)))))))

(event `ShowInventorylist`
  (for _array_element (`self.DatatableItems`)
    (`KismetSystemLibrary.PrintString` (`KismetStringLibrary.Conv_NameToString` (`.ChestID_8_BFBAAD3F4112D46E9C599BBFA1B441CD` (break `/Game/Structure/S_ChestData` _array_element))))))