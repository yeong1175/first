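; Player interaction component that finds interactable actors in front of its owner and triggers their item interaction.
; A looping timer runs a short forward sphere trace, keeping hits that implement Bpi_Interaction as HitActor and showing their look-at message in the player HUD, clearing it otherwise.
; The interaction input prints a debug "Hello" and calls InteractWith on the target's BPC_Itemdata component, passing the owner.
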(event `self.ReceiveBeginPlay`
  (`KismetSystemLibrary.K2_SetTimerDelegate` (delegate `UpdateInteraction`) 0.1 true))

(event `UpdateInteraction`
  (`self.InteractionTrace`))

(event `EnhancedInput|/Game/TopDown/Input/Actions/IA_Interaction`
  (params (ActionValue :type Boolean) (ElapsedSeconds :type "Float (double-precision)") (TriggeredSeconds :type "Float (double-precision)") (InputAction :type "InputAction Object Reference" :default "/Game/TopDown/Input/Actions/IA_Interaction.IA_Interaction"))
  (:`Started`
    (bind _hit_actor (`self.Hit Actor`)
      (:`then`
        (`KismetSystemLibrary.PrintString` "Hello")
        (bind _returnvalue (`Actor.GetComponentByClass` _hit_actor "/Game/UtubeInventory/ItemData/BPC_Itemdata.BPC_Itemdata_C"))
        (`/Engine/EditorBlueprintResources/StandardMacros.IsValid` _returnvalue
          (:`Is Valid`
            (`/Game/UtubeInventory/Interaction/Interaction/Bpi_Interaction.InteractWith` _returnvalue (`self.GetOwner`)))))
      (:`else`))))

(fn `GetInteractionUI`
  (returns (WB_Interaction_UI_36 :type "/Game/UtubeInventory/Interaction/UI/Mui/WB_Interaction_UI Object Reference"))
  (bind _asbp_fight_third_person_player_controller (cast `/Game/ThirdPerson/Blueprints/BP_FightThirdPerson/BP_FightThirdPersonPlayerController` (`GameplayStatics.GetPlayerController` 0)))
  (return (`/Game/UtubeInventory/Interaction/WB_PlayerHud.WB_Interaction_UI_36` (`/Game/ThirdPerson/Blueprints/BP_FightThirdPerson/BP_FightThirdPersonPlayerController.WB_PlayerHud` _asbp_fight_third_person_player_controller))))

(fn `InteractionTrace`
  (bind _returnvalue (`self.GetOwner`))
  (bind _returnvalue_2 (`Actor.K2_GetActorLocation` _returnvalue))
  ; Comment
  (bind (_outhit _returnvalue_3) (`KismetSystemLibrary.SphereTraceSingle` :`Start` _returnvalue_2 :`End` (+ _returnvalue_2 (* (`Actor.GetActorForwardVector` _returnvalue) 100.0)) :`Radius` 70.0 :`TraceChannel` "TraceTypeQuery4" :`DrawDebugType` "ForOneFrame"))
  (if _returnvalue_3
    (bind (_bblockinghit _binitialoverlap _time _distance _location _impactpoint _normal _impactnormal _physmat _hitactor) (`GameplayStatics.BreakHitResult` _outhit))
    (if (`KismetSystemLibrary.DoesImplementInterface` _hitactor "/Game/UtubeInventory/Interaction/Interaction/Bpi_Interaction.Bpi_Interaction_C")
      (bind _output_get (set `self.Hit Actor` _hitactor))
      (bind _message (message `/Game/UtubeInventory/Interaction/Interaction/Bpi_Interaction.Lookat` _output_get))
      (`/Game/UtubeInventory/Interaction/UI/Mui/WB_Interaction_UI.SetMessage` (`self.GetInteractionUI`) _message)
      (else
        (set `self.Hit Actor` null)
        (`/Game/UtubeInventory/Interaction/UI/Mui/WB_Interaction_UI.SetMessage` (`self.GetInteractionUI`) "")))
    (else
      (set `self.Hit Actor` null)
      (`/Game/UtubeInventory/Interaction/UI/Mui/WB_Interaction_UI.SetMessage` (`self.GetInteractionUI`) ""))))